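; BP_AIHostage is an AI hostage that moves to the player on sight and is picked up on contact.
; Its PawnSensing component sets a visibility flag when it sees a pawn, then issues an AI Move To toward the player character.
; When the player overlaps its box collider, it notifies BP_GameMode through OnPickUp and destroys itself.
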(event OnSeePawn(PawnSensing)
  (params (Pawn :type Pawn%20Object%20Reference))
  (Variables|Default|SetisPlayerVisible true)
  (CallFunction|Move2Player))

(event OnComponentBeginOverlap(BoxCollider)
  (params (OverlappedComponent :type Primitive%20Component%20Object%20Reference) (OtherActor :type Actor%20Object%20Reference) (OtherComp :type Primitive%20Component%20Object%20Reference) (OtherBodyIndex :type Integer) (bFromSweep :type Boolean) (SweepResult :type Hit%20Result%20Structure%20%28by%20ref%29))
  ;[0 0.167 1] Player Collider Check
  (if (== OtherActor (Game|GetPlayerCharacter 0))
    (bind _asbp_game_mode (Utilities|Casting|CastToBP_GameMode (Game|GetGameMode)))
    (Default|OnPickUp _asbp_game_mode)
    (Actor|DestroyActor)))

(event Custom|Move2Player
  (if (Variables|Default|GetisPlayerVisible)
    (AI|AIMoveTo self "0, 0, 0" (Game|GetPlayerCharacter 0) 5.0 false)))

(fn ConstructionScript)