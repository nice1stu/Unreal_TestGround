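; Player controller for the Intro content that handles respawning and switching the player into another character.
; RespawnCharacter unpossesses the current pawn, spawns a fresh BP_Character at the given location and rotation, and possesses it.
; AddEnterable and RemoveEnterable set and clear a single enterable character reference.
; EnterNewCharacter checks that reference, destroys the current player character and possesses the stored one.
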(event Custom|RespawnCharacter
  (params (Spawn%20Transform%20Location :type Vector) (Spawn%20Transform%20Rotation :type Rotator))
  ;[0.0612 1 0] Respawn Character
  (Pawn|UnPossess)
  (bind _returnvalue (Game|SpawnActorfromClass "/Game/Intro/Blueprints/BP_Character.BP_Character_C" (Math|Transform|MakeTransform Spawn%20Transform%20Location Spawn%20Transform%20Rotation "1.000000,1.000000,1.000000") "Undefined" "MultiplyWithRoot" 0 0))
  (Pawn|Possess _returnvalue))

(event Custom|AddEnterable
  (params (Character%20is%20Enterable :type Character%20Object%20Reference))
  (Variables|Default|SetCharacter%20Is%20Enterable Character%20is%20Enterable))

(event Custom|EnterNewCharacter
  (bind _character_is_enterable (Variables|Default|GetCharacter%20Is%20Enterable)
    (:then
      (Actor|DestroyActor (Game|GetPlayerCharacter 0))
      (Pawn|Possess _character_is_enterable))
    (:else)))

(event Custom|RemoveEnterable
  (Variables|Default|SetCharacter%20Is%20Enterable 0))

(fn ConstructionScript)