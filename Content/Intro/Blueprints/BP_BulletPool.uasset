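; Bullet pool that pre-spawns BP_Bullet actors for its owner, so they can be reused.
; On BeginPlay it spawns bullets at the owner's location, disables their mesh collision, attaches them to the owner and stores them in the BulletPool array.
; Each bullet's OnBulletDestroyed dispatcher is bound to ReturnToPool, which only moves the bullet back to the owner and reattaches it.
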(event Custom|ReturnToPool
  (params (Bullets :type BP%20Bullet%20Object%20Reference))
  (bind _returnvalue (Components|GetOwner))
  (Transformation|SetActorLocation Bullets (Transformation|GetActorLocation _returnvalue) false false)
  (Transformation|AttachActorToActor Bullets _returnvalue "None" "KeepWorld" "KeepWorld" "KeepWorld" true))

(event EventBeginPlay
  (for _index (range 0 (Variables|Default|GetAmountOfBullets))
    (bind _returnvalue (Game|SpawnActorfromClass "/Game/Intro/Blueprints/BP_Bullet.BP_Bullet_C" (Math|Transform|MakeTransform (Transformation|GetActorLocation (Components|GetOwner)) "0, 0, 0" "1.000000,1.000000,1.000000") "Undefined" "MultiplyWithRoot" 0 0))
    (Collision|SetCollisionEnabled (Variables|/Game/Intro/Blueprints/BP_Bullet.BP_Bullet_C|GetBulletMesh _returnvalue) "NoCollision")
    (Transformation|AttachActorToActor _returnvalue (Components|GetOwner) "None" "KeepWorld" "KeepWorld" "KeepWorld" true)
    (EventDispatchers|AssignOnBulletDestroyed _returnvalue (delegate Custom|ReturnToPool))
    (Utilities|Array|Add (Variables|Default|GetBulletPool) _returnvalue)))