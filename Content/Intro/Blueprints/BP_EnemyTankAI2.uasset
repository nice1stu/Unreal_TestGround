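; Enemy tank AI that chases the player once its tank PawnSensing component spots a pawn.
; A sighting sets a visibility flag and calls AIMoveTo toward player character 0; nothing clears the flag.
; The turret sensing event is empty, leaving the chopper cast, zero-valued rotation and shooting branch unwired.
; The Enemy Shooting macro holds delayed, impulse-launched projectile spawning, but its input is also disconnected, so the tank never fires.
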(event OnSeePawn(PawnSensingTank)
  (params (Pawn :type Pawn%20Object%20Reference))
  ;[0 0.2046 1] Move Towards Player
  (Variables|Default|SetisPlayerVisible true)
  (CallFunction|Move2Player))

(event OnSeePawn(PawnSensingTurret)
  (params (Pawn :type Pawn%20Object%20Reference))
  ;[1 0.009947 0] Turret Face Player and Shoot
)

(event Custom|Move2Player
  ;[0 0.2046 1] Move Towards Player
  (if (Variables|Default|GetisPlayerVisible)
    (AI|AIMoveTo self "0, 0, 0" (Game|GetPlayerCharacter 0) 5.0 false)))

(fn ConstructionScript)